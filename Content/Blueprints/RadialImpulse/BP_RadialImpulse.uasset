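; Radial impulse Blueprint that drives the visuals of a burst: an expanding ring and a depleted-to-full color change.
; ExpandRing plays the Morpher timeline to scale the Ring and set the passed dynamic material's opacity.
; MorphBaseColor picks a 2, 3 or 4 second timeline from BurstFrequency bands to lerp BaseColor, and plays none above the top band.
; The file shows no impulse logic or callers for either event.
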(event `self.ExpandRing`
  (params (MID :type "MaterialInstanceDynamic Object Reference"))
  (if (`KismetSystemLibrary.IsValid` MID)
    (bind (_direction _size _opacity) (`Timeline|Morpher` :!via `PlayFromStart`)
      (:`Update`
        (`SceneComponent.SetRelativeScale3D` (`self.Ring`) (`KismetMathLibrary.VLerp` (`self.Small`) (`self.Big`) _size))
        (`MaterialInstanceDynamic.SetScalarParameterValue` MID "Opacity" _opacity)))))

(event `self.MorphBaseColor`
  (params (MID :type "MaterialInstanceDynamic Object Reference"))
  (bind _burstfrequency (`self.BurstFrequency`))
  (if (`KismetSystemLibrary.IsValid` MID)
    (`/Engine/EditorBlueprintResources/StandardMacros.CompareFloat` _burstfrequency 2.9
      (:`>`
        (`/Engine/EditorBlueprintResources/StandardMacros.CompareFloat` _burstfrequency 3.9
          (:`>`
            (`/Engine/EditorBlueprintResources/StandardMacros.CompareFloat` _burstfrequency 4.9
              (:`<`
                (bind (_direction _4sec) (`Timeline|4_Sec` :!via `PlayFromStart`)
                  (:`Update`
                    (`MaterialInstanceDynamic.SetVectorParameterValue` MID "BaseColor" (`KismetMathLibrary.LinearColorLerp` (`self.Color_Depleted`) (`self.Color_Full`) _4sec)))))))
          (:`<`
            (bind (_direction_2 _3sec) (`Timeline|3_Sec` :!via `PlayFromStart`)
              (:`Update`
                (`MaterialInstanceDynamic.SetVectorParameterValue` MID "BaseColor" (`KismetMathLibrary.LinearColorLerp` (`self.Color_Depleted`) (`self.Color_Full`) _3sec)))))))
      (:`<`
        (bind (_direction_3 _morph2sec) (`Timeline|2 Sec` :!via `PlayFromStart`)
          (:`Update`
            (`MaterialInstanceDynamic.SetVectorParameterValue` MID "BaseColor" (`KismetMathLibrary.LinearColorLerp` (`self.Color_Depleted`) (`self.Color_Full`) _morph2sec))))))))

(fn `UserConstructionScript`)