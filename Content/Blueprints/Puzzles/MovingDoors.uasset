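; Puzzle door Blueprint that moves its Door component between an upper and a lower relative location.
; MoveDoor1Down and MoveDoor1Up each drive their own timeline, lerping between DoorOneUpper and DoorOneLower in opposite directions without sweep.
; Tick alternates the two events through a FlipFlop, so each timeline restarts from the beginning every other frame rather than waiting to finish.
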(event `self.ReceiveTick`
  (params (DeltaSeconds :type "Float (single-precision)"))
  (`/Engine/EditorBlueprintResources/StandardMacros.FlipFlop`
    (:`A`
      (`self.MoveDoor1Down`))
    (:`B`
      (`self.MoveDoor1Up`))))

(event `MoveDoor1Down`
  (bind (_direction _door1down) (`Timeline|Timeline_0` :!via `PlayFromStart`)
    (:`Update`
      (`SceneComponent.K2_SetRelativeLocation` (`self.Door`) (`KismetMathLibrary.VLerp` (`self.DoorOneUpper`) (`self.DoorOneLower`) _door1down) false false))))

(event `MoveDoor1Up`
  (bind (_direction _door1down) (`Timeline|Timeline_1` :!via `PlayFromStart`)
    (:`Update`
      (`SceneComponent.K2_SetRelativeLocation` (`self.Door`) (`KismetMathLibrary.VLerp` (`self.DoorOneLower`) (`self.DoorOneUpper`) _door1down) false false))))

(fn `UserConstructionScript`)