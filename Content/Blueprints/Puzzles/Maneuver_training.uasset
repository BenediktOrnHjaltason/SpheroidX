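; Tutorial maneuvering puzzle that leads the player through a chain of eight key pickups to open a door.
; On BeginPlay it caches the child-actor keys, leaving only the first visible and collidable.
; Each key's overlap reveals the next in a fixed, non-numeric order.
; The last overlap plays a timeline that lerps the door to its destination and clears the tutorial game mode's IsInTutorial1 flag.
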(event `OnComponentBeginOverlap_Event_6`
  (params (OverlappedComponent :type "PrimitiveComponent Object Reference") (OtherActor :type "Actor Object Reference") (OtherComp :type "PrimitiveComponent Object Reference") (OtherBodyIndex :type Integer) (bFromSweep :type Boolean) (SweepResult :type "HitResult Structure (by ref)"))
  (bind _bp_key5 (`self.BP_Key5`))
  (`self.SetActorHiddenInGame` _bp_key5 false)
  (`self.SetActorEnableCollision` _bp_key5 true))

(event `OnComponentBeginOverlap_Event_4`
  (params (OverlappedComponent :type "PrimitiveComponent Object Reference") (OtherActor :type "Actor Object Reference") (OtherComp :type "PrimitiveComponent Object Reference") (OtherBodyIndex :type Integer) (bFromSweep :type Boolean) (SweepResult :type "HitResult Structure (by ref)"))
  (bind _bp_key8 (`self.BP_Key8`))
  (`self.SetActorHiddenInGame` _bp_key8 false)
  (`self.SetActorEnableCollision` _bp_key8 true))

(event `OnComponentBeginOverlap_Event_5`
  (params (OverlappedComponent :type "PrimitiveComponent Object Reference") (OtherActor :type "Actor Object Reference") (OtherComp :type "PrimitiveComponent Object Reference") (OtherBodyIndex :type Integer) (bFromSweep :type Boolean) (SweepResult :type "HitResult Structure (by ref)"))
  (bind _bp_key4 (`self.BP_Key4`))
  (`self.SetActorHiddenInGame` _bp_key4 false)
  (`self.SetActorEnableCollision` _bp_key4 true))

(event `OnComponentBeginOverlap_Event_7`
  (params (OverlappedComponent :type "PrimitiveComponent Object Reference") (OtherActor :type "Actor Object Reference") (OtherComp :type "PrimitiveComponent Object Reference") (OtherBodyIndex :type Integer) (bFromSweep :type Boolean) (SweepResult :type "HitResult Structure (by ref)"))
  (`self.OpenDoor`)
  (set `/Game/Blueprints/GameModes/BP_GameMode_Tutorial.IsInTutorial1` false (`self.GameMode_Tutoial_Ref`)))

(event `OnComponentBeginOverlap_Event_3`
  (params (OverlappedComponent :type "PrimitiveComponent Object Reference") (OtherActor :type "Actor Object Reference") (OtherComp :type "PrimitiveComponent Object Reference") (OtherBodyIndex :type Integer) (bFromSweep :type Boolean) (SweepResult :type "HitResult Structure (by ref)"))
  (bind _bp_key2 (`self.BP_Key2`))
  (`self.SetActorHiddenInGame` _bp_key2 false)
  (`self.SetActorEnableCollision` _bp_key2 true))

(event `self.ReceiveBeginPlay`
  (bind _asbp_game_mode_tutorial (cast `/Game/Blueprints/GameModes/BP_GameMode_Tutorial` (`GameplayStatics.GetGameMode`)))
  (set `self.GameMode_Tutoial_Ref` _asbp_game_mode_tutorial)
  (`self.SetupTutorial1`)
  (add `PrimitiveComponent.OnComponentBeginOverlap` (`PickupBase.Collision` (`self.BP_Key1`)) (delegate `OnComponentBeginOverlap_Event_0`))
  (add `PrimitiveComponent.OnComponentBeginOverlap` (`PickupBase.Collision` (`self.BP_Key6`)) (delegate `OnComponentBeginOverlap_Event_1`))
  (add `PrimitiveComponent.OnComponentBeginOverlap` (`PickupBase.Collision` (`self.BP_Key7`)) (delegate `OnComponentBeginOverlap_Event_2`))
  (add `PrimitiveComponent.OnComponentBeginOverlap` (`PickupBase.Collision` (`self.BP_Key3`)) (delegate `OnComponentBeginOverlap_Event_3`))
  (add `PrimitiveComponent.OnComponentBeginOverlap` (`PickupBase.Collision` (`self.BP_Key2`)) (delegate `OnComponentBeginOverlap_Event_4`))
  (add `PrimitiveComponent.OnComponentBeginOverlap` (`PickupBase.Collision` (`self.BP_Key8`)) (delegate `OnComponentBeginOverlap_Event_5`))
  (add `PrimitiveComponent.OnComponentBeginOverlap` (`PickupBase.Collision` (`self.BP_Key4`)) (delegate `OnComponentBeginOverlap_Event_6`))
  (add `PrimitiveComponent.OnComponentBeginOverlap` (`PickupBase.Collision` (`self.BP_Key5`)) (delegate `OnComponentBeginOverlap_Event_7`)))

(event `OnComponentBeginOverlap_Event_2`
  (params (OverlappedComponent :type "PrimitiveComponent Object Reference") (OtherActor :type "Actor Object Reference") (OtherComp :type "PrimitiveComponent Object Reference") (OtherBodyIndex :type Integer) (bFromSweep :type Boolean) (SweepResult :type "HitResult Structure (by ref)"))
  (bind _bp_key3 (`self.BP_Key3`))
  (`self.SetActorHiddenInGame` _bp_key3 false)
  (`self.SetActorEnableCollision` _bp_key3 true))

(event `OnComponentBeginOverlap_Event_0`
  (params (OverlappedComponent :type "PrimitiveComponent Object Reference") (OtherActor :type "Actor Object Reference") (OtherComp :type "PrimitiveComponent Object Reference") (OtherBodyIndex :type Integer) (bFromSweep :type Boolean) (SweepResult :type "HitResult Structure (by ref)"))
  (bind _bp_key6 (`self.BP_Key6`))
  (`self.SetActorHiddenInGame` _bp_key6 false)
  (`self.SetActorEnableCollision` _bp_key6 true))

(event `OnComponentBeginOverlap_Event_1`
  (params (OverlappedComponent :type "PrimitiveComponent Object Reference") (OtherActor :type "Actor Object Reference") (OtherComp :type "PrimitiveComponent Object Reference") (OtherBodyIndex :type Integer) (bFromSweep :type Boolean) (SweepResult :type "HitResult Structure (by ref)"))
  (bind _bp_key7 (`self.BP_Key7`))
  (`self.SetActorHiddenInGame` _bp_key7 false)
  (`self.SetActorEnableCollision` _bp_key7 true))

(event `OpenDoor`
  (bind (_direction _newtrack_0) (`Timeline|OpenDoorYeah` :!via `PlayFromStart`)
    (:`Update`
      (`SceneComponent.K2_SetRelativeLocation` (`self.Door`) (`KismetMathLibrary.VLerp` (`self.DoorLocation`) (`self.DoorDestination`) _newtrack_0) false false))))

(fn `SetupTutorial1`
  (bind _asbp_pickup_key (cast `/Game/Blueprints/Pickups/Keys/BP_Pickup_Key` (`ChildActorComponent.ChildActor` (`self.Key1`))))
  (bind _output_get (set `self.BP_Key1` _asbp_pickup_key))
  (`self.SetActorHiddenInGame` _output_get false)
  (`self.SetActorEnableCollision` _output_get true)
  (bind _asbp_pickup_key_2 (cast `/Game/Blueprints/Pickups/Keys/BP_Pickup_Key` (`ChildActorComponent.ChildActor` (`self.Key2`))))
  (bind _output_get_2 (set `self.BP_Key2` _asbp_pickup_key_2))
  (`self.SetActorHiddenInGame` _output_get_2 true)
  (`self.SetActorEnableCollision` _output_get_2 false)
  (bind _asbp_pickup_key_3 (cast `/Game/Blueprints/Pickups/Keys/BP_Pickup_Key` (`ChildActorComponent.ChildActor` (`self.Key3`))))
  (bind _output_get_3 (set `self.BP_Key3` _asbp_pickup_key_3))
  (`self.SetActorHiddenInGame` _output_get_3 true)
  (`self.SetActorEnableCollision` _output_get_3 false)
  (bind _asbp_pickup_key_4 (cast `/Game/Blueprints/Pickups/Keys/BP_Pickup_Key` (`ChildActorComponent.ChildActor` (`self.Key4`))))
  (bind _output_get_4 (set `self.BP_Key4` _asbp_pickup_key_4))
  (`self.SetActorHiddenInGame` _output_get_4 true)
  (`self.SetActorEnableCollision` _output_get_4 false)
  (bind _asbp_pickup_key_5 (cast `/Game/Blueprints/Pickups/Keys/BP_Pickup_Key` (`ChildActorComponent.ChildActor` (`self.Key5`))))
  (bind _output_get_5 (set `self.BP_Key5` _asbp_pickup_key_5))
  (`self.SetActorHiddenInGame` _output_get_5 true)
  (`self.SetActorEnableCollision` _output_get_5 false)
  (bind _asbp_pickup_key_6 (cast `/Game/Blueprints/Pickups/Keys/BP_Pickup_Key` (`ChildActorComponent.ChildActor` (`self.Key6`))))
  (bind _output_get_6 (set `self.BP_Key6` _asbp_pickup_key_6))
  (`self.SetActorHiddenInGame` _output_get_6 true)
  (`self.SetActorEnableCollision` _output_get_6 false)
  (bind _asbp_pickup_key_7 (cast `/Game/Blueprints/Pickups/Keys/BP_Pickup_Key` (`ChildActorComponent.ChildActor` (`self.Key7`))))
  (bind _output_get_7 (set `self.BP_Key7` _asbp_pickup_key_7))
  (`self.SetActorHiddenInGame` _output_get_7 true)
  (`self.SetActorEnableCollision` _output_get_7 false)
  (bind _asbp_pickup_key_8 (cast `/Game/Blueprints/Pickups/Keys/BP_Pickup_Key` (`ChildActorComponent.ChildActor` (`self.Key8`))))
  (bind _output_get_8 (set `self.BP_Key8` _asbp_pickup_key_8))
  (`self.SetActorHiddenInGame` _output_get_8 true)
  (`self.SetActorEnableCollision` _output_get_8 false)
  (return))

(fn `UserConstructionScript`)