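; BP_Accelerator is an accelerator actor that can spin around its roll axis and play a sound effect.
; On BeginPlay, if ShouldRotate is set, Start sets a looping timer that calls AddRotation by name every Frequency seconds, stepping world roll by DegreesToTurn instead of using Tick.
; A separate PlaySoundEffect event plays the Accelerator sound in 2D and has no caller in this graph.
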(event `self.ReceiveBeginPlay`
  (if (`self.bShouldRotate`)
    (`self.Start`)))

(event `AddRotation`
  (`self.K2_AddActorWorldRotation` (`KismetMathLibrary.MakeRotator` (`self.DegreesToTurn`))))

(event `self.PlaySoundEffect`
  (`GameplayStatics.PlaySound2D` "/Game/Sound/Accelerator.Accelerator" 1.0 1.0 0.0 null null))

(fn `Start`
  (`KismetSystemLibrary.K2_SetTimer` null "AddRotation" (`self.Frequency`) true))

(fn `UserConstructionScript`)