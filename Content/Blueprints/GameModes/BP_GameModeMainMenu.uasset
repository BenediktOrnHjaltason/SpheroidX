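; Main menu game mode that prepares saved progress and shows the menu when play begins.
; On BeginPlay it caches the BP_GameInstance and loads level times from disk unless ResetAllTimes is set.
; An UnlockAllLevels flag overwrites every entry in the instance's LevelsLocked array.
; It then enables player input, adds the main menu widget to the viewport and plays the menu sound cue.
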(event `self.ReceiveBeginPlay`
  (bind _levelslocked (`SpheroidGameInstance.LevelsLocked` (`self.GameInstanceRef`)))
  (bind _asbp_game_instance (cast `/Game/Blueprints/BP_GameInstance` (`GameplayStatics.GetGameInstance`)))
  (bind _output_get (set `self.GameInstanceRef` _asbp_game_instance))
  (if (not (`self.bResetAllTimes`))
    (`SpheroidGameInstance.LoadLevelTimesFromDisk` _output_get))
  (`self.EnableInput` (`GameplayStatics.GetPlayerController` 0) null)
  (if (`self.bUnlockAllLevels`)
    (for (_ _array_index) _levelslocked
      (`KismetArrayLibrary.Array_Set` _levelslocked _array_index)))
  (bind _returnvalue (`|CreateWidget` "/Game/Blueprints/UI/MainMenuWidget.MainMenuWidget_C"))
  (`UserWidget.AddToViewport` _returnvalue 0)
  (set `self.MainMenuWidget` _returnvalue)
  (`GameplayStatics.PlaySound2D` "/Game/Sound/MainMenuCue.MainMenuCue" 1.0 1.0 0.0 null null))

(fn `UserConstructionScript`)