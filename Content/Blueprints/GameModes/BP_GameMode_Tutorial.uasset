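; Tutorial game mode that resets the active tutorial puzzle when notified of a death.
; In the first tutorial it sets up the maneuver training puzzle again and clears the Spheroid's key count.
; In the second tutorial it passes the death to the stay-still puzzle's own handler.
; Begin play only calls the parent implementation.
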(event `self.ReceiveBeginPlay`
  (`parent.ReceiveBeginPlay`))

(event `self.NotifiedOfDeath`
  (if (`self.IsInTutorial1`)
    (`/Game/Blueprints/Puzzles/Maneuver_training.SetupTutorial1` (`self.Puzzle_ManeuverTraining`))
    (set `Avatar.Keys` 0 (`self.Spheroid`))
    (elif (`self.IsInTutorial2`)
      (`/Game/Blueprints/Puzzles/StayStill.StayStill_OnDeath` (`self.Puzzle_StayStill`)))))

(fn `UserConstructionScript`
  (`parent.UserConstructionScript`))