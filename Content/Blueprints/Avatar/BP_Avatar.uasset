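; BP_Avatar is the player avatar, providing timeline-driven movement and effects plus the level transition screen.
; Custom events play timelines for entrance movement, death, boost, momentum stop and portal morph, feeding values into functions defined outside these graphs, or directly into mesh scale.
; DisplayTime creates a tutorial or regular transition widget, passing level references to the latter.
; LerpCamera is an empty event, with its camera timeline logic left disconnected.
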(event `self.ReceiveBeginPlay`
  (`self.EnableInput` (`GameplayStatics.GetPlayerController` 0)))

(event `self.TL_MoveToEntrance`
  (bind (_direction _movetoentrance) (`Timeline|MoveToEntrance` :!via `PlayFromStart`)
    (:`Update`
      (`self.MoveToEntrance` _movetoentrance))
    (:`Finished`
      (`self.AfterMove`))))

(event `self.TL_DeathEffect`
  (`SpheroidXGameModeBase.PlayCameraShake` (`self.GameModeRef`) "Death")
  (`GameplayStatics.PlaySound2D` "/Game/Sound/Death.Death" 1.0 1.0 0.0 null null)
  (bind (_direction _scale) (`Timeline|DeathEffect` :!via `PlayFromStart`)
    (:`Update`
      (`self.DeathEffect` _scale))
    (:`Finished`
      (`self.EffectCleanUp`))))

(event `self.TL_BoostEffect`
  (bind (_direction _scale _opacity) (`Timeline|Boost` :!via `PlayFromStart`)
    (:`Update`
      (`self.BoostEffect` _scale _opacity))
    (:`Finished`
      (`self.EffectCleanUp` :!label _label))))

(event `self.TL_StopMomentumEffect`
  (bind (_direction _scale) (`Timeline|StopMomentum` :!via `PlayFromStart`)
    (:`Update`
      (`self.StopMomentumEffect` _scale))
    (:`Finished`
      (goto _label))))

(event `self.PortalMorph`
  (bind (_direction _morphscale) (`Timeline|TL_PortalMorph` :!via `PlayFromStart`)
    (:`Update`
      (`SceneComponent.SetRelativeScale3D` (`self.PlaneMesh`) (`KismetMathLibrary.VLerp` (`self.PortalMorphBig`) (`self.PortalMorphSmall`) _morphscale)))
    (:`Finished`
      (`self.PortalMorphCleanUp`))))

(event `self.DisplayTime`
  (if (`self.bIsTutorialLevel`)
    (bind _returnvalue (`|CreateWidget` "/Game/Blueprints/UI/LevelTransitionsBasicTraining.LevelTransitionsBasicTraining_C"))
    (`UserWidget.AddToViewport` _returnvalue 0)
    (else
      (bind _returnvalue_2 (`|CreateWidget` "/Game/Blueprints/UI/LevelTransitionsWidget.LevelTransitionsWidget_C"))
      (`UserWidget.AddToViewport` _returnvalue_2 0)
      (set `/Game/Blueprints/UI/LevelTransitionsWidget.PreviousLevel` (`self.PreviousLevel`) _returnvalue_2)
      (set `/Game/Blueprints/UI/LevelTransitionsWidget.CurrentLevel` (`self.CurrentLevel`) _returnvalue_2)
      (set `/Game/Blueprints/UI/LevelTransitionsWidget.NextLevel` (`self.NextLevel`) _returnvalue_2)
      (if (`self.bIsFirstLevel`)
        (`/Game/Blueprints/UI/LevelTransitionsWidget.RemoveButton_PreviousLevel` _returnvalue_2)))))

(event `self.LerpCamera`
  (params (LocationAtDirectionChange :type "Vector Structure") (TowardsPosition :type "Vector Structure")))

(fn `UserConstructionScript`)